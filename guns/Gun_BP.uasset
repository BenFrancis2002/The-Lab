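; Grabbable VR gun actor that fires Bullet actors.
; Pickup, called by BP_MotionController, disables mesh physics, snaps the root to the given component and applies a fixed grip offset to the mesh.
; Drop restores physics and detaches the gun in place.
; Shooting spawns a Bullet at the Arrow component's world location, without passing the Arrow's rotation.
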(event `/Game/VirtualRealityBP/Blueprints/PickupActorInterface.Pickup`
  (params (AttachTo :type "SceneComponent Object Reference"))
  (`PrimitiveComponent.SetSimulatePhysics` (`self.StaticMeshComponent`) false)
  (`SceneComponent.K2_AttachToComponent` (`self.K2_GetRootComponent`) AttachTo "None" "SnapToTarget" "SnapToTarget" "KeepWorld" false)
  (`SceneComponent.K2_SetRelativeLocationAndRotation` (`self.StaticMeshComponent`) (-0.000358 19.0 -8.0) (struct :`Yaw` 180.0) false false))

(event `/Game/VirtualRealityBP/Blueprints/PickupActorInterface.Drop`
  (`PrimitiveComponent.SetSimulatePhysics` (`self.StaticMeshComponent`) true)
  (`self.K2_DetachFromActor` "KeepWorld" "KeepWorld" "KeepWorld"))

(fn `shooting`
  (`|SpawnActorFromClass` "/Game/guns/bullet.bullet_C" (`KismetMathLibrary.MakeTransform` (`SceneComponent.K2_GetComponentLocation` (`self.Arrow`))) "Undefined" "OverrideRootScale" null null))

(fn `UserConstructionScript`)